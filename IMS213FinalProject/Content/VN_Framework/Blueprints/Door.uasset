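; Door actor that slides its mesh upward once enough items have been collected.
; CollectItem increments a counter, and opendoorcheck compares it to the required total, then calls OpenDoor once through a DoOnce.
; OpenDoor plays a timeline that lerps the mesh's relative Z height while keeping X, Y and scale.
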(event `open door`
  (bind _staticmesh1 (`self.StaticMesh1`))
  (bind (_relativelocation_x _relativelocation_y) (`KismetMathLibrary.BreakVector` (`SceneComponent.RelativeLocation` _staticmesh1)))
  (bind (_direction _door_up) (`Timeline|opening door`)
    (:`Update`
      (`SceneComponent.K2_SetRelativeTransform` _staticmesh1 (`KismetMathLibrary.MakeTransform` (`KismetMathLibrary.MakeVector` _relativelocation_x _relativelocation_y (`KismetMathLibrary.Lerp` 0.0 450.0 _door_up)) (struct) (`SceneComponent.RelativeScale3D` _staticmesh1)) false false))))

(event `Collect Item`
  (`/Engine/EditorBlueprintResources/StandardMacros.IncrementInt` (`self.currentitemscollected`)))

(event `open door check`
  (if (>= (`self.currentitemscollected`) (`self.maxitemscollected`))
    (`/Engine/EditorBlueprintResources/StandardMacros.DoOnce` false
      (:`Completed`
        (`self.open door`)))))

(fn `UserConstructionScript`)